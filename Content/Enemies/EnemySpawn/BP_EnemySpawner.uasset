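; BP_EnemySpawner is a placeable spawner that creates enemies once the player's progress reaches a kill threshold.
; On BeginPlay it reads KillCount from BP_GameInstance and compares it to AmountOfKills, with no later re-check.
; If the threshold is met, SpawnEnemy loops to spawn NumberOfEnemies of the configured Enemy class, all at the spawner's own transform.
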(event `self.ReceiveBeginPlay`
  (bind _asbp_game_instance (cast `/Game/BP_GameInstance` (`GameplayStatics.GetGameInstance`)))
  (set `self.As BP Game Instance` _asbp_game_instance)
  (if (>= (`/Game/BP_GameInstance.KillCount` (`self.As BP Game Instance`)) (`self.AmountOfKills`))
    (`self.SpawnEnemy` (`self.Enemy`) (`self.GetTransform`) (`self.Number Of Enemies`))))

(event `SpawnEnemy`
  (params (Enemy :type "Actor Class Reference") (SpawnTransform :type "Transform Structure") (NumberOfEnemies :type Integer))
  (for _ (range NumberOfEnemies)
    (`|SpawnActorFromClass` Enemy SpawnTransform "Undefined" "MultiplyWithRoot" null null)))

(fn `UserConstructionScript`)