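; Camera actor that becomes the player's view target and follows the player character at a fixed Z height.
; Each tick, GetNewXValue and GetNewYValue move the camera only when the character leaves a per-axis dead zone around it, keeping it at that zone's edge.
; The construction script, when a follow actor is already set, places the camera at a fixed offset and pitches it toward that actor.
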(event `self.ReceiveBeginPlay`
  (set `self.ActorToFollow` (`GameplayStatics.GetPlayerCharacter` 0))
  (`PlayerController.SetViewTargetWithBlend` (`GameplayStatics.GetPlayerController` 0) self 0.0 "VTBlend_Linear" 0.0 false))

(event `self.ReceiveTick`
  (params (DeltaSeconds :type "Float (single-precision)"))
  (bind _newx (`self.GetNewXValue`))
  (set `self.CameraX` _newx)
  (bind _newy (`self.GetNewYValue`))
  (set `self.CameraY` _newy)
  (`self.K2_SetActorLocation` (`KismetMathLibrary.MakeVector` (`self.CameraX`) (`self.CameraY`) (`self.ZOffset`))))

(fn `GetNewXValue`
  (returns (NewX :type "Float (double-precision)"))
  (bind _returnvalue_x (`KismetMathLibrary.BreakVector` (`self.K2_GetActorLocation`)))
  (bind _returnvalue_x_2 (`KismetMathLibrary.BreakVector` (`self.K2_GetActorLocation`)))
  (bind _returnvalue_x_3 (`KismetMathLibrary.BreakVector` (`self.K2_GetActorLocation` (`self.ActorToFollow`))))
  (bind _returnvalue_x_4 (`KismetMathLibrary.BreakVector` (`self.K2_GetActorLocation` (`self.ActorToFollow`))))
  (bind _returnvalue (- _returnvalue_x_4 (`self.XDeadZone`)))
  (bind _returnvalue_2 (+ _returnvalue_x_3 (`self.XDeadZone`)))
  (if (> _returnvalue _returnvalue_x_2)
    (return _returnvalue)
    (elif (< _returnvalue_2 _returnvalue_x)
      (return _returnvalue_2)
      (else
        (return (`self.CameraX`))))))

(fn `GetNewYValue`
  (returns (NewY :type "Float (double-precision)"))
  (bind (_returnvalue_x _returnvalue_y) (`KismetMathLibrary.BreakVector` (`self.K2_GetActorLocation`)))
  (bind (_returnvalue_x_2 _returnvalue_y_2) (`KismetMathLibrary.BreakVector` (`self.K2_GetActorLocation`)))
  (bind (_returnvalue_x_3 _returnvalue_y_3) (`KismetMathLibrary.BreakVector` (`self.K2_GetActorLocation` (`self.ActorToFollow`))))
  (bind (_returnvalue_x_4 _returnvalue_y_4) (`KismetMathLibrary.BreakVector` (`self.K2_GetActorLocation` (`self.ActorToFollow`))))
  (bind _returnvalue (+ _returnvalue_y_4 (`self.YDeadZone`)))
  (bind _returnvalue_2 (- _returnvalue_y_3 (`self.YDeadZone`)))
  (if (< _returnvalue _returnvalue_y_2)
    (return _returnvalue)
    (elif (> _returnvalue_2 _returnvalue_y)
      (return _returnvalue_2)
      (else
        (return (`self.CameraY`))))))

(fn `UserConstructionScript`
  (bind _actortofollow (`self.ActorToFollow`))
  (bind (_returnvalue_x _returnvalue_y) (`KismetMathLibrary.BreakVector` (`self.K2_GetActorLocation` _actortofollow)))
  (bind (_returnvalue_roll _returnvalue_pitch) (`KismetMathLibrary.BreakRotator` (`KismetMathLibrary.FindLookAtRotation` (`self.K2_GetActorLocation`) (`self.K2_GetActorLocation` (`self.ActorToFollow`)))))
  (`/Engine/EditorBlueprintResources/StandardMacros.IsValid` _actortofollow
    (:`Is Valid`
      (bind _output_get (set `self.CameraX` (- _returnvalue_x 30.0)))
      (bind _output_get_2 (set `self.CameraY` (- _returnvalue_y 50.0)))
      (`self.K2_SetActorLocation` (`KismetMathLibrary.MakeVector` _output_get _output_get_2 (`self.ZOffset`)))
      (`self.K2_SetActorRotation` (`KismetMathLibrary.MakeRotator` 0.0 _returnvalue_pitch)))))