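; Room camera actor that becomes the view target and BP_Franky's CurrentCam when Franky overlaps its trigger box, including at BeginPlay.
; The construction script places the trigger and sizes the confine box from RoomWidth and RoomHeight.
; BeginPlay derives clamp limits from that box, inset by half of Width and Length.
; Every Tick, the camera interpolates toward Franky in X and Y, clamped to those limits, keeping Z unchanged.
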(event `self.ReceiveBeginPlay`
  (`self.GetConfinesBoxBounds`
    (:`Out`
      (`KismetSystemLibrary.Delay` 0.0)
      (bind _asbp_franky (cast `/Game/Character/BP_Franky` (`GameplayStatics.GetPlayerPawn` 0)))
      (for _array_element (`self.GetOverlappingComponents` _asbp_franky)
        (if (== _array_element (`self.Player Trigger Box`))
          (set `/Game/Character/BP_Franky.CurrentCam` self _asbp_franky)
          (`PlayerController.SetViewTargetWithBlend` (`GameplayStatics.GetPlayerController` 0) self 0.0 "VTBlend_Linear" 0.0 false))))))

(event `self.Player Trigger Box.OnComponentBeginOverlap`
  (params (OverlappedComponent :type "PrimitiveComponent Object Reference") (OtherActor :type "Actor Object Reference") (OtherComp :type "PrimitiveComponent Object Reference") (OtherBodyIndex :type Integer) (bFromSweep :type Boolean) (SweepResult :type "HitResult Structure (by ref)"))
  (bind _asbp_franky (cast `/Game/Character/BP_Franky` OtherActor))
  (set `/Game/Character/BP_Franky.CurrentCam` self _asbp_franky)
  (`PlayerController.SetViewTargetWithBlend` (`GameplayStatics.GetPlayerController` 0) self 0.0 "VTBlend_Linear" 0.0 false))

(event `self.ReceiveTick`
  (params (DeltaSeconds :type "Float (single-precision)"))
  (bind (_returnvalue_x _returnvalue_y _returnvalue_z) (`KismetMathLibrary.BreakVector` (`SceneComponent.K2_GetComponentLocation` (`self.Camera`))))
  (set `self.Delta Time` DeltaSeconds)
  (`self.CamFollowPlayerX`
    (:`Out`
      (`self.CamFollowPlayerY`
        (:`Out`
          (`self.LerpWithinConfines`
            (:`Out`
              (`SceneComponent.K2_SetWorldLocation` (`self.Camera`) (`KismetMathLibrary.MakeVector` (`self.CameraX`) (`self.CameraY`) _returnvalue_z) false false))))))))

(fn `UserConstructionScript`
  (`SceneComponent.K2_SetRelativeTransform` (`self.Player Trigger Box`) (`self.Player Trigger Transform`) false false)
  (`BoxComponent.SetBoxExtent` (`self.Player Trigger Box`) (`self.Player Trigger Extent `) true)
  (`BoxComponent.SetBoxExtent` (`self.CollisionConfineBox`) (`KismetMathLibrary.MakeVector` (`KismetMathLibrary.Conv_IntToDouble` (* (`self.RoomWidth`) 575)) (`KismetMathLibrary.Conv_IntToDouble` (* (`self.RoomHeight`) 325)) 50.0) true))