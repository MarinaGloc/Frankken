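; Camera actor that becomes the player's view target on BeginPlay, built to follow the player character outside a map-centred dead zone.
; Per-axis check events compare player position to map-centre offsets, though both read player X and use only greater-than tests.
; Passing checks move the actor by VInterpTo toward the player on that axis and Z.
; Start/Stop events toggle a Tick gate, but its output drives nothing and neither check is called here.
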(event `self.ReceiveBeginPlay`
  (`PlayerController.SetViewTargetWithBlend` (`GameplayStatics.GetPlayerController` 0) self 0.0 "VTBlend_Linear" 0.0 false)
  (`self.StartCamFollow`))

(event `self.ReceiveTick`
  (params (DeltaSeconds :type "Float (single-precision)"))
  (`/Engine/EditorBlueprintResources/StandardMacros.Gate` true :!label _label))

(event `StartCamFollow`
  (goto _label :!via `Open`))

(event `StopCamFollow`
  (goto _label :!via `Close`))

(event `CheckPlayerX`
  (bind _returnvalue_x (`KismetMathLibrary.BreakVector` (`self.K2_GetActorLocation` (`GameplayStatics.GetPlayerCharacter` 0))))
  (bind _returnvalue_x_2 (`KismetMathLibrary.BreakVector` (`self.K2_GetActorLocation` (`GameplayStatics.GetPlayerCharacter` 0))))
  (if (and (> _returnvalue_x (+ (`self.MapCenterX`) (`self.MinX`))) (> _returnvalue_x_2 (+ (`self.MapCenterX`) (`self.MaxX`))))
    (`self.MoveCameraX`)))

(event `MoveCameraX`
  (bind (_returnvalue_x _returnvalue_y) (`KismetMathLibrary.BreakVector` (`self.K2_GetActorLocation`)))
  (bind (_returnvalue_x_2 _returnvalue_y_2 _returnvalue_z) (`KismetMathLibrary.BreakVector` (`self.K2_GetActorLocation` (`GameplayStatics.GetPlayerCharacter` 0))))
  (`self.K2_SetActorLocation` (`KismetMathLibrary.VInterpTo` (`self.K2_GetActorLocation`) (`KismetMathLibrary.MakeVector` _returnvalue_x_2 _returnvalue_y _returnvalue_z) (`GameplayStatics.GetWorldDeltaSeconds`))))

(event `CheckPlayerY`
  (bind _returnvalue_x (`KismetMathLibrary.BreakVector` (`self.K2_GetActorLocation` (`GameplayStatics.GetPlayerCharacter` 0))))
  (bind _returnvalue_x_2 (`KismetMathLibrary.BreakVector` (`self.K2_GetActorLocation` (`GameplayStatics.GetPlayerCharacter` 0))))
  (if (and (> _returnvalue_x_2 (+ (`self.MapCenterY`) (`self.MinY`))) (> _returnvalue_x (+ (`self.MapCenterY`) (`self.MaxY`))))
    (`self.MoveCameraY`)))

(event `MoveCameraY`
  (bind _returnvalue_x (`KismetMathLibrary.BreakVector` (`self.K2_GetActorLocation`)))
  (bind (_returnvalue_x_2 _returnvalue_y _returnvalue_z) (`KismetMathLibrary.BreakVector` (`self.K2_GetActorLocation` (`GameplayStatics.GetPlayerCharacter` 0))))
  (`self.K2_SetActorLocation` (`KismetMathLibrary.VInterpTo` (`self.K2_GetActorLocation`) (`KismetMathLibrary.MakeVector` _returnvalue_x _returnvalue_y _returnvalue_z) (`GameplayStatics.GetWorldDeltaSeconds`))))

(fn `UserConstructionScript`)