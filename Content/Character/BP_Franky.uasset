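; Franky is the player character, with world-axis movement, melee attacks and health, driven by Enhanced Input.
; BeginPlay adds health bar and kill-count widgets outside menu, intro and end levels; attacking zeroes walk speed while held.
; HitDetect sphere-traces around Franky to trigger an enemy's HitReact.
; Franky's own HitReact applies delay-gated damage, or on death notifies BP_GM, reopens Level1, resets kills and requests a restart.
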(event `self.ReceiveBeginPlay`
  (`|ExecutionSequence`
    (:`then_0`
      (bind _asplayer_controller (cast `PlayerController` (`self.GetController`)))
      (`EnhancedInputSubsystemInterface.AddMappingContext` (pcsubsystem `EnhancedInputLocalPlayerSubsystem` _asplayer_controller) "/Game/Character/Input/IMC_Franky.IMC_Franky" 0 (struct)))
    (:`then_1`
      (bind _returnvalue (`GameplayStatics.GetCurrentLevelName` true))
      (if (not (or (== _returnvalue "MainMenu") (== _returnvalue "Intro") (== _returnvalue "End")))
        (bind _returnvalue_2 (`|CreateWidget` "/Game/UI/HealthBar.HealthBar_C"))
        (bind _output_get (set `self.HealthBarWG` _returnvalue_2))
        (`UserWidget.AddToViewport` _output_get 0)
        (bind _returnvalue_3 (`|CreateWidget` "/Game/UI/KillCountWG.KillCountWG_C"))
        (`UserWidget.AddToViewport` _returnvalue_3 0)))))

(event `EnhancedInput|/Game/Character/Input/IA_Move`
  (params (ActionValue :type "Vector2D Structure") (ElapsedSeconds :type "Float (double-precision)") (TriggeredSeconds :type "Float (double-precision)") (InputAction :type "InputAction Object Reference" :default "/Game/Character/Input/IA_Move.IA_Move"))
  (:`Triggered`
    (if (not (`self.IsDead`))
      (`self.AddMovementInput` (1.0 0.0 0.0) ActionValue_X)
      (`self.AddMovementInput` (0.0 -1.0 0.0) ActionValue_Y)
      (set `self.Directionality` (`KismetMathLibrary.MakeVector2D` ActionValue_X ActionValue_Y))))
  (:`Started`
    (set `self.IsHoldingMove` true))
  (:`Completed`
    (set `self.IsHoldingMove` false)))

(event `EnhancedInput|/Game/Character/Input/IA_Attack`
  (params (ActionValue :type Boolean) (ElapsedSeconds :type "Float (double-precision)") (TriggeredSeconds :type "Float (double-precision)") (InputAction :type "InputAction Object Reference" :default "/Game/Character/Input/IA_Attack.IA_Attack"))
  (:`Started`
    (set `self.IsAttacking` true)
    (set `CharacterMovementComponent.MaxWalkSpeed` 0.0 (`self.CharacterMovement`)))
  (:`Completed`
    (set `self.IsAttacking` false)
    (set `CharacterMovementComponent.MaxWalkSpeed` 400.0 (`self.CharacterMovement`))))

(event `HitReact`
  (if (not (`self.GettingHit`))
    (set `self.GettingHit` true)
    (if (<= (`self.Health`) 0.0)
      (set `self.IsDead` true)
      (`KismetSystemLibrary.Delay` 0.4)
      (`self.Destroy`)
      (`GameplayStatics.OpenLevel` "Level1_Map")
      (bind _asbp_game_instance (cast `/Game/BP_GameInstance` (`GameplayStatics.GetGameInstance`)))
      (set `/Game/BP_GameInstance.KillCount` 0 _asbp_game_instance)
      (`self.CallRestartPlayer`)
      (else
        (bind _output_get (set `self.Health` (- (`self.Health`) (`self.Damage Amount`))))
        (set `/Game/UI/HealthBar.Health` _output_get (`self.HealthBarWG`))
        (`KismetSystemLibrary.Delay` 0.5)
        (set `self.GettingHit` false)))))

(event `Destroy`
  (bind _asbp_gm (cast `/Game/BP_GM` (`GameplayStatics.GetGameMode`)))
  (`/Game/BP_GM.On Player Died` _asbp_gm self))

(fn `CallRestartPlayer`
  (locals (ControllerRef :type "Controller Object Reference"))
  (set `local.ControllerRef` (`self.GetController`))
  (`self.K2_DestroyActor`)
  (bind _asbp_gm (cast `/Game/BP_GM` (`GameplayStatics.GetGameMode`)))
  (`GameModeBase.RestartPlayer` _asbp_gm (`local.ControllerRef`)))

(fn `HitDetect`
  (bind _returnvalue (`self.K2_GetActorLocation`))
  (bind _outhit (`KismetSystemLibrary.SphereTraceSingleForObjects` :`Start` _returnvalue :`End` _returnvalue :`Radius` 45.0 :`ObjectTypes` (`|MakeArray` "ObjectTypeQuery3" :!type "EObjectTypeQuery Enum") :`DrawDebugType` "ForDuration"))
  (bind _asai_enemy (cast `/Game/Enemies/AI_Enemy` (`.HitActor` (`GameplayStatics.BreakHitResult` _outhit))))
  (`/Game/Enemies/AI_Enemy.HitReact` _asai_enemy))

(fn `IsStuck`
  (returns (IsStuck :type Boolean))
  (return (and (`self.IsHoldingMove`) (< (`KismetMathLibrary.VSize` (`self.GetVelocity`)) (`self.Stuck Thresholde`)))))

(fn `UserConstructionScript`)